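; BP_Pig is a pig character that turns around when it meets a wall or reaches a ledge.
; An overlap on WallDetector triggers a 180-degree rotation.
; Each tick, while the current floor is walkable, it also rotates if the LedgeDector component overlaps no actors, using that empty overlap as the sign of a drop ahead.
; The file itself adds no movement input.
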(event OnComponentBeginOverlap(WallDetector)
  (params (OverlappedComponent :type Primitive%20Component%20Object%20Reference) (OtherActor :type Actor%20Object%20Reference) (OtherComp :type Primitive%20Component%20Object%20Reference) (OtherBodyIndex :type Integer) (bFromSweep :type Boolean) (SweepResult :type Hit%20Result%20Structure%20%28by%20ref%29))
  (CallFunction|FRotateCharacter))

(event EventTick
  (params (DeltaSeconds :type Float%20%28single-precision%29))
  (|CallParentFunction DeltaSeconds)
  (CallFunction|FCheckLedge))

(fn ConstructionScript
  (|CallParentFunction))

(fn FRotateCharacter
  (Transformation|SetActorRotation (Math|Rotator|CombineRotators (Transformation|GetActorRotation) "0.000000,180.000000,0.000000")))

(fn FCheckLedge
  (if (.bwalkablefloor (Variables|/Script/Engine.CharacterMovementComponent|GetCurrentFloor (Variables|Character|GetCharacterMovement)))
    (if (not (> (Utilities|Array|Length (Collision|GetOverlappingActors (Variables|Default|GetLedgeDector) 0 :!class /Script/Engine.PrimitiveComponent)) 0))
      (CallFunction|FRotateCharacter))))